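; LeapPawn_BP is a pawn that visualises Leap Motion hand tracking with debug drawing.
; On BeginPlay it optimises the Leap controller for HMD top-down use.
; Each tick it reads the current frame, prints the hand count, and draws spheres at stabilised palm positions and fingertips, shifted by a fixed world offset rather than the pawn's location.
; Fingers are fetched with GetPointableById using the loop index as the ID.
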(event EventBeginPlay
  (Class|LeapController|OptimizeforHMD (Variables|Default|GetLeapController) true true true))

(event Collision|EventActorBeginOverlap
  (params (OtherActor :type Actor%20Object%20Reference)))

(event EventTick
  (params (DeltaSeconds :type Float%20%28single-precision%29))
  (bind _returnvalue (Class|LeapController|Frame (Variables|Default|GetLeapController)))
  (bind _returnvalue_2 (Class|LeapFrame|Hands _returnvalue))
  (Development|PrintText (Utilities|Text|ToText(Integer) (Variables|/Script/LeapMotion.LeapHandList|GetCount _returnvalue_2)) true true "(R=1.000000,G=0.000000,B=0.017360,A=1.000000)" 0.0)
  (if (not (Variables|/Script/LeapMotion.LeapHandList|GetIsEmpty _returnvalue_2))
    (for _index (range 0 (- (Variables|/Script/LeapMotion.LeapHandList|GetCount _returnvalue_2) 1))
      (bind _returnvalue_3 (Class|LeapHandList|GetIndex _returnvalue_2 _index))
      (Rendering|Debug|DrawDebugSphere (+ (Variables|/Script/LeapMotion.LeapHand|GetStabilizedPalmPosition _returnvalue_3) "-180.000000, 0,150.000000") 1.0 5 "(R=0.000000,G=0.620000,B=0.019107,A=1.000000)" 0.0 0.5)
      (bind _returnvalue_4 (Class|LeapHand|Fingers _returnvalue_3))
      (for _index_2 (range 0 (- (Variables|/Script/LeapMotion.LeapFingerList|GetCount _returnvalue_4) 1))
        (bind _returnvalue_5 (Class|LeapFingerList|GetPointablebyId _returnvalue_4 _index_2))
        (Rendering|Debug|DrawDebugSphere (+ (Variables|/Script/LeapMotion.LeapPointable|GetTipPosition _returnvalue_5) "-180.000000, 0,150.000000") 1.0 5 "(R=0.000000,G=0.620000,B=0.019107,A=1.000000)" 0.0 0.5)))))

(fn ConstructionScript)