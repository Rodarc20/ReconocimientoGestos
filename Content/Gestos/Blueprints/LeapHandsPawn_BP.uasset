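; Pawn that reads hand data from a Leap Motion controller, optimized for HMD use, to classify gestures.
; BeginPlay loads the ClasificadorGestos database, and GrabarBaseDatos writes it.
; Capturar calibrates a middle-finger-to-palm reference distance from the first detected hand.
; Once calibrated, Clasfificar feeds fingertip-to-palm distances normalized by that reference into the classifier, printing the result and drawing debug spheres.
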(event EventBeginPlay
  (Class|ClasificadorGestos|CargarBase (Variables|Default|GetClasificadorGestos))
  (Class|LeapController|OptimizeforHMD (Variables|Default|GetLeapController) true true true))

(event Collision|EventActorBeginOverlap
  (params (OtherActor :type Actor%20Object%20Reference)))

(event EventTick
  (params (DeltaSeconds :type Float%20%28single-precision%29)))

(event Input|ActionEvents|InputActionCapturar
  (params (Key :type Key%20Structure :default "LeapLeftPinch"))
  (:Pressed
    (bind _returnvalue (Class|LeapController|Frame (Variables|Default|GetLeapController)))
    (bind _returnvalue_2 (Class|LeapFrame|Hands _returnvalue))
    (if (not (Variables|/Script/LeapMotion.LeapHandList|GetIsEmpty _returnvalue_2))
      (bind _returnvalue_3 (Class|LeapHandList|GetIndex _returnvalue_2))
      (bind _returnvalue_4 (Class|LeapHand|Fingers _returnvalue_3))
      (bind _returnvalue_5 (Class|LeapFingerList|GetPointablebyId _returnvalue_4 2))
      (bind _output_get (Variables|Default|SetDistanciaMedio (Math|Vector|VectorLength (- (Variables|/Script/LeapMotion.LeapPointable|GetTipPosition _returnvalue_5) (Variables|/Script/LeapMotion.LeapHand|GetPalmPosition _returnvalue_3)))))
      (Development|PrintText (Utilities|Text|ToText(Float) _output_get "HalfToEven") true true "(R=0.009809,G=0.625000,B=0.106367,A=1.000000)" 0.5))))

(event Input|ActionEvents|InputActionClasfificar
  (params (Key :type Key%20Structure :default "LeapLeftPinch"))
  (:Pressed
    (if (!= (Variables|Default|GetDistanciaMedio) 0.0)
      (Class|ClasificadorGestos|BorrarMano (Variables|Default|GetClasificadorGestos))
      (bind _returnvalue (Class|LeapController|Frame (Variables|Default|GetLeapController)))
      (bind _returnvalue_2 (Class|LeapFrame|Hands _returnvalue))
      (if (not (Variables|/Script/LeapMotion.LeapHandList|GetIsEmpty _returnvalue_2))
        (bind _returnvalue_3 (Class|LeapHandList|GetIndex _returnvalue_2))
        (bind _returnvalue_4 (Class|LeapHand|Fingers _returnvalue_3))
        (for _index (range 0 (- (Variables|/Script/LeapMotion.LeapFingerList|GetCount _returnvalue_4) 1))
          (bind _returnvalue_5 (Class|LeapFingerList|GetPointablebyId _returnvalue_4 _index))
          (Class|ClasificadorGestos|AgregarDistanciaDedo (Variables|Default|GetClasificadorGestos) (/ (Math|Vector|VectorLength (- (Variables|/Script/LeapMotion.LeapPointable|GetTipPosition _returnvalue_5) (Variables|/Script/LeapMotion.LeapHand|GetPalmPosition _returnvalue_3))) (Variables|Default|GetDistanciaMedio)))
          (Development|PrintText (Utilities|Text|ToText(Float) (.X (Math|Vector|BreakVector (Variables|/Script/LeapMotion.LeapPointable|GetTipPosition _returnvalue_5))) "HalfToEven") true true "(R=0.000000,G=0.660000,B=1.000000,A=1.000000)" 0.0)
          (Development|PrintText (Utilities|Text|ToText(Float) (.Y (Math|Vector|BreakVector (Variables|/Script/LeapMotion.LeapPointable|GetTipPosition _returnvalue_5))) "HalfToEven") true true "(R=0.000000,G=0.660000,B=1.000000,A=1.000000)" 0.0)
          (Development|PrintText (Utilities|Text|ToText(Float) (.Z (Math|Vector|BreakVector (Variables|/Script/LeapMotion.LeapPointable|GetTipPosition _returnvalue_5))) "HalfToEven") true true "(R=0.000000,G=0.660000,B=1.000000,A=1.000000)" 0.0)
          (Rendering|Debug|DrawDebugSphere (+ (Variables|/Script/LeapMotion.LeapPointable|GetTipPosition _returnvalue_5) "-180.000000, 0,150.000000") 2.0 5 "(R=0.000000,G=0.034457,B=1.000000,A=1.000000)" 2.0 1.0)
          (Rendering|Debug|DrawDebugSphere (+ (Variables|/Script/LeapMotion.LeapHand|GetStabilizedPalmPosition _returnvalue_3) "-180.000000, 0,150.000000") 2.0 5 "(R=0.000000,G=0.034457,B=1.000000,A=1.000000)" 2.0 1.0))
        (bind _returnvalue_6 (Class|ClasificadorGestos|ClasificarMano (Variables|Default|GetClasificadorGestos)))
        (Development|PrintText (Utilities|Text|ToText(Integer) _returnvalue_6) true true "(R=0.009809,G=0.625000,B=0.106367,A=1.000000)" 1.0)))))

(event Input|ActionEvents|InputActionGrabarBaseDatos
  (params (Key :type Key%20Structure :default "LeapLeftPinch"))
  (:Pressed
    (Class|ClasificadorGestos|EscribirBase (Variables|Default|GetClasificadorGestos))))

(fn ConstructionScript
  (|CallParentFunction))